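; Basic pepperbox gun actor that acts as the player's first-person view model for weapon slot 3.
; Each Tick it reads WeaponSelected from FirstPersonCharacter and shows the mesh only when that slot is active.
; While active, it moves itself to a fixed forward, right and down offset from the camera, deriving roll from camera pitch and offsetting yaw to align the mesh.
; It contains no firing logic.
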(event EventBeginPlay)

(event Collision|EventActorBeginOverlap
  (params (OtherActor :type Actor%20Object%20Reference)))

(event EventTick
  (params (DeltaSeconds :type Float%20%28single-precision%29))
  (bind _returnvalue (Game|GetPlayerController 0))
  (bind _playercameramanager (Variables|/Script/Engine.PlayerController|GetPlayerCameraManager _returnvalue))
  (bind _returnvalue_2 (Camera|GetCameraRotation _playercameramanager))
  (bind (_roll _pitch _yaw) (Math|Rotator|BreakRotator _returnvalue_2))
  (bind _result (Math|Float|NegateFloat _pitch)
    (:%20%20
      (bind _asfirst_person_character (Utilities|Casting|CastToFirstPersonCharacter (Game|GetPlayerCharacter 0))
        (:then
          _)
        (:CastFailed
          _))
      ;[1 1 1] If weapon selected == 3, this weapon
      (Rendering|SetVisibility (Variables|Default|GetPepperBox_Mesh_01c) (== (Variables|/Game/FirstPersonBP/Blueprints/FirstPersonCharacter.FirstPersonCharacter_C|GetweaponSelected _asfirst_person_character) 3) true)
      (if (== (Variables|/Game/FirstPersonBP/Blueprints/FirstPersonCharacter.FirstPersonCharacter_C|GetweaponSelected _asfirst_person_character) 3)
        (Transformation|SetActorTransform (Math|Transform|MakeTransform (+ (Transformation|GetActorLocation (Game|GetPlayerCameraManager 0)) (* (Math|Vector|Normalize (Math|Vector|GetForwardVector _returnvalue_2)) 5e+01) (* (Math|Vector|Normalize (Math|Vector|GetRightVector _returnvalue_2)) 25.0) (* (Math|Vector|Normalize (Math|Vector|GetUpVector _returnvalue_2)) -2e+01)) (Math|Rotator|MakeRotator _result 0.0 (- _yaw 9e+01))))))))

(fn ConstructionScript)