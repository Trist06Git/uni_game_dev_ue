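; A basic enemy actor that moves along the world X axis.
; Each Tick adds Speed to its X location without sweep or delta-time scaling, so movement depends on frame rate, and resets scale to one.
; A frame counter periodically triggers an operation on Speed, apparently a sign flip for back-and-forth patrol, then restarts.
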(event EventBeginPlay)

(event Collision|EventActorBeginOverlap
  (params (OtherActor :type Actor%20Object%20Reference)))

(event EventTick
  (params (DeltaSeconds :type Float%20%28single-precision%29))
  (bind _returnvalue (Transformation|GetActorLocation))
  (bind (_x _y _z) (Math|Vector|BreakVector _returnvalue))
  (Transformation|SetActorTransform (Math|Transform|MakeTransform (Math|Vector|MakeVector (+ _x (Math|Conversions|ToFloat(Integer) (Variables|Default|Getspeed))) _y _z) (Transformation|GetActorRotation)))
  (Variables|Default|Setframes (+ (Variables|Default|Getframes) 1))
  (if (>= (Variables|Default|Getframes) 100)
    (Utilities|NegateInt (Variables|Default|Getspeed)
      (:%20%20
        (Variables|Default|Setframes 0)))))

(fn ConstructionScript)